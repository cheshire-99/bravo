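; BP_DamageNotify is an animation notify state that marks the window in which the character's sword is active, likely for dealing damage.
; On begin and on end, it casts the mesh owner to BP_TopDownCharacter and gets the BP_Weapon from its Weapon child actor component.
; It calls SwordActive when the window opens and SwordDeactive when it closes.
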(fn `Received_NotifyBegin`
  (params (MeshComp :type "SkeletalMeshComponent Object Reference") (Animation :type "AnimSequenceBase Object Reference") (TotalDuration :type "Float (single-precision)") (EventReference :type "AnimNotifyEventReference Structure (by ref)"))
  (returns (ReturnValue :type Boolean))
  (bind _asbp_top_down_character (cast `/Game/TopDown/Blueprints/BP_TopDownCharacter` (`ActorComponent.GetOwner` MeshComp)))
  (bind _asbp_weapon (cast `/Game/bravo/Charactor/Blueprints/BP_Weapon` (`ChildActorComponent.ChildActor` (`/Game/TopDown/Blueprints/BP_TopDownCharacter.Weapon` _asbp_top_down_character))))
  (`/Game/bravo/Charactor/Blueprints/BP_Weapon.Sword Active` _asbp_weapon)
  (return false))

(fn `Received_NotifyEnd`
  (params (MeshComp :type "SkeletalMeshComponent Object Reference") (Animation :type "AnimSequenceBase Object Reference") (EventReference :type "AnimNotifyEventReference Structure (by ref)"))
  (returns (ReturnValue :type Boolean))
  (bind _asbp_top_down_character (cast `/Game/TopDown/Blueprints/BP_TopDownCharacter` (`ActorComponent.GetOwner` MeshComp)))
  (bind _asbp_weapon (cast `/Game/bravo/Charactor/Blueprints/BP_Weapon` (`ChildActorComponent.ChildActor` (`/Game/TopDown/Blueprints/BP_TopDownCharacter.Weapon` _asbp_top_down_character))))
  (`/Game/bravo/Charactor/Blueprints/BP_Weapon.Sword Deactive` _asbp_weapon)
  (return false))