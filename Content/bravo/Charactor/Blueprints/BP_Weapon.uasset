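; BP_Weapon is a sword weapon actor that applies SwordDamage to actors overlapping its WeaponCollision component.
; SwordActive and SwordDeactive switch the hitbox on with an OverlapAll profile and off with NoCollision.
; The overlap handler compares the overlapped component, rather than the other actor, to the owner.
; Damage passes through a DoOnce with no visible reset, and the trailing half-second Delay leads nowhere.
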(event `self.WeaponCollision.OnComponentBeginOverlap`
  (params (OverlappedComponent :type "PrimitiveComponent Object Reference") (OtherActor :type "Actor Object Reference") (OtherComp :type "PrimitiveComponent Object Reference") (OtherBodyIndex :type Integer) (bFromSweep :type Boolean) (SweepResult :type "HitResult Structure (by ref)"))
  (if (!= OverlappedComponent (`self.GetOwner`))
    (`/Engine/EditorBlueprintResources/StandardMacros.DoOnce` false
      (:`Completed`
        (`GameplayStatics.ApplyDamage` OtherActor (`self.SwordDamage`))
        (`KismetSystemLibrary.Delay` 0.5)))))

(event `Sword Active`
  (`PrimitiveComponent.SetCollisionProfileName` (`self.WeaponCollision`) "OverlapAll" true))

(event `Sword Deactive`
  (`PrimitiveComponent.SetCollisionEnabled` (`self.WeaponCollision`) "NoCollision"))

(fn `UserConstructionScript`)