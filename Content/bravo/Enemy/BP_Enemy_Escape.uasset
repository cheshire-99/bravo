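; Enemy Blueprint that handles health, damage and death; no escape behavior appears in its graphs.
; Damage passes through a resettable DoOnce, lowers Health and refreshes the overhead WBP_unit_Health bar against a fixed maximum.
; On death it disables capsule collision and movement, ragdolls mesh, head and wheel, then hides them with a bail-out Niagara effect before destruction.
; It also credits player character 0 with experience and a defeat count.
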(event `self.ReceiveBeginPlay`
  (bind _aswbp_unit_health (cast `/Game/bravo/Enemy/WBP_unit_Health` (`WidgetComponent.GetUserWidgetObject` (`self.unit_hpbar`))))
  (`/Game/bravo/Enemy/WBP_unit_Health.UpdateHealth` _aswbp_unit_health (/ (`self.health`) 150.0)))

(event `self.ReceiveAnyDamage`
  (params (Damage :type "Float (single-precision)") (DamageType :type "DamageType Object Reference") (InstigatedBy :type "Controller Object Reference") (DamageCauser :type "Actor Object Reference"))
  (bind _returnvalue (`GameplayStatics.GetPlayerCharacter` 0))
  (`/Engine/EditorBlueprintResources/StandardMacros.DoOnce` false :!label _label
    (:`Completed`
      (if (> (`self.health`) 0.0)
        (set `self.health` (- (`self.health`) Damage))
        (`|ExecutionSequence`
          (:`then_0`
            (bind _aswbp_unit_health (cast `/Game/bravo/Enemy/WBP_unit_Health` (`WidgetComponent.GetUserWidgetObject` (`self.unit_hpbar`))))
            (`/Game/bravo/Enemy/WBP_unit_Health.UpdateHealth` _aswbp_unit_health (/ (`self.health`) 150.0))
            (goto _label :!via `Reset`))
          (:`then_1`
            (if (<= (`self.health`) 0.0)
              (`|ExecutionSequence`
                (:`then_0`
                  (`PrimitiveComponent.SetCollisionEnabled` (`self.CapsuleComponent`) "NoCollision")
                  ;[1 1 1] 倒されたら、見えなくして消失エフェクトを表示
                  (`CharacterMovementComponent.DisableMovement` (`self.CharacterMovement`))
                  (`PrimitiveComponent.SetSimulatePhysics` (`self.Mesh`) true)
                  (`PrimitiveComponent.SetSimulatePhysics` (`self.head`) true)
                  (`PrimitiveComponent.SetSimulatePhysics` (`self.wheel`) true)
                  (`KismetSystemLibrary.Delay` 2.0)
                  (`SceneComponent.SetVisibility` (`self.Mesh`) false false)
                  (`SceneComponent.SetVisibility` (`self.head`) false false)
                  (`SceneComponent.SetVisibility` (`self.wheel`) false false)
                  (`NiagaraFunctionLibrary.SpawnSystemAttached` "/Game/bravo/Enemy/VFX/NS_BailOut.NS_BailOut" (`self.Mesh`) "None" (0.0 0.0 0.0) (struct) "SnapToTarget")
                  (`KismetSystemLibrary.Delay` 4.0)
                  (`self.K2_DestroyActor`))
                (:`then_1`
                  ;[1 1 1] 敵を倒したActorに経験値+1
                  (bind _asbp_top_down_character (cast `/Game/TopDown/Blueprints/BP_TopDownCharacter` _returnvalue))
                  (`/Game/TopDown/Blueprints/BP_TopDownCharacter.get_Exp` _asbp_top_down_character)
                  (set `self.isDeath?` true))
                (:`then_2`
                  ;[1 1 1] 敵を倒したら倒した数を更新
                  (bind _asbp_top_down_character_2 (cast `/Game/TopDown/Blueprints/BP_TopDownCharacter` _returnvalue))
                  (`/Game/TopDown/Blueprints/BP_TopDownCharacter.UpdateDefeatsEnemy` _asbp_top_down_character_2)
                  (`KismetSystemLibrary.Delay` 0.5)
                  (goto _label :!via `Reset`))))))))))

(fn `UserConstructionScript`)