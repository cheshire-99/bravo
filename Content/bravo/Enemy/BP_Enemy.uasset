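; Enemy character that attacks the player, takes damage and rewards the player when killed.
; Attack damage and interval come from DT_EnemyData, with ChangeParam advancing to the next row.
; Attack plays a montage whose notify sphere-traces for a Player-tagged pawn, then waits out the interval.
; Damage updates the health bar and spawns damage text; death ragdolls the parts, credits experience and a defeat, plays a Niagara effect and destroys the actor.
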(event `ChangeParam`
  (set `self.EnemyData` (+ (`self.EnemyData`) 1))
  (bind _returnvalue (`|GetDataTableRow` "/Game/bravo/Enemy/EnemyData/DT_EnemyData.DT_EnemyData" (`KismetStringLibrary.Conv_StringToName` (`KismetStringLibrary.Conv_IntToString` (`self.EnemyData`))))
    (:`then`
      (set `self.AttackDamage` (break `/Game/bravo/Enemy/EnemyData/ST_EnemyData` _returnvalue))
      (set `self.AttackWait` (`.AttackInterval_4_E418C91D46CA98D2E01B7CBC46050ACB` (break `/Game/bravo/Enemy/EnemyData/ST_EnemyData` _returnvalue)))
      (`KismetSystemLibrary.PrintString` (`KismetStringLibrary.Conv_IntToString` (`self.EnemyData`))))))

(event `self.ReceiveBeginPlay`
  (bind _aswbp_unit_health (cast `/Game/bravo/Enemy/WBP_unit_Health` (`WidgetComponent.GetUserWidgetObject` (`self.unit_hpbar`))))
  (`/Game/bravo/Enemy/WBP_unit_Health.UpdateHealth` _aswbp_unit_health (/ (`self.health`) 100.0))
  (bind _returnvalue (`|GetDataTableRow` "/Game/bravo/Enemy/EnemyData/DT_EnemyData.DT_EnemyData" (`KismetStringLibrary.Conv_StringToName` (`KismetStringLibrary.Conv_IntToString` (`self.EnemyData`))))
    (:`then`
      (set `self.AttackDamage` (break `/Game/bravo/Enemy/EnemyData/ST_EnemyData` _returnvalue))
      (set `self.AttackWait` (`.AttackInterval_4_E418C91D46CA98D2E01B7CBC46050ACB` (break `/Game/bravo/Enemy/EnemyData/ST_EnemyData` _returnvalue)))
      (`KismetSystemLibrary.PrintString` (`KismetStringLibrary.Conv_IntToString` (`self.EnemyData`))))))

(event `/Game/bravo/Enemy/BPI_EnemyFight.Attack`
  (bind _attackpos (`self.AttackPos`))
  (bind _returnvalue (`SceneComponent.K2_GetComponentLocation` _attackpos))
  ;[1 1 1] Attack
  (if (and (not (`self.isAttacking?`)) (not (`self.isDeath?`)))
    ;;[1 1 1] Select Animation -> Montage + set Montage 23:28
    (`|PlayMontage` (`self.Mesh`) "/Game/bravo/Ancient_Golem/Demo/ThirdPersonJump_Start_Montage.ThirdPersonJump_Start_Montage"
      (:`then`
        (set `self.isAttacking?` true))
      (:`OnCompleted`
        (`KismetSystemLibrary.Delay` (`self.AttackWait`))
        (set `self.isAttacking?` false))
      (:`OnNotifyBegin`
        (bind (_outhit _returnvalue_2) (`KismetSystemLibrary.SphereTraceSingleForObjects` :`Start` _returnvalue :`End` (+ _returnvalue (* (`KismetMathLibrary.GetForwardVector` (`SceneComponent.K2_GetComponentRotation` _attackpos)) 150.0)) :`Radius` 10.0 :`ObjectTypes` (`|MakeArray` "ObjectTypeQuery3" :!type "EObjectTypeQuery Enum") :`DrawDebugType` "ForDuration" :`DrawTime` 2.0))
        (if _returnvalue_2
          (bind (_bblockinghit _binitialoverlap _time _distance _location _impactpoint _normal _impactnormal _physmat _hitactor) (`GameplayStatics.BreakHitResult` _outhit))
          (if (`self.ActorHasTag` _hitactor "Player")
            (`GameplayStatics.ApplyDamage` _hitactor (`self.AttackDamage`))))))))

(event `self.ReceiveAnyDamage`
  (params (Damage :type "Float (single-precision)") (DamageType :type "DamageType Object Reference") (InstigatedBy :type "Controller Object Reference") (DamageCauser :type "Actor Object Reference"))
  (bind _returnvalue (`GameplayStatics.GetPlayerCharacter` 0))
  (`/Engine/EditorBlueprintResources/StandardMacros.DoOnce` false :!label _label
    (:`Completed`
      (if (> (`self.health`) 0.0)
        (set `self.health` (- (`self.health`) Damage))
        (`|ExecutionSequence`
          (:`then_0`
            (bind _aswbp_unit_health (cast `/Game/bravo/Enemy/WBP_unit_Health` (`WidgetComponent.GetUserWidgetObject` (`self.unit_hpbar`))))
            (`/Game/bravo/Enemy/WBP_unit_Health.UpdateHealth` _aswbp_unit_health (/ (`self.health`) 100.0))
            (goto _label :!via `Reset`))
          (:`then_1`
            (if (<= (`self.health`) 0.0)
              (`|ExecutionSequence`
                (:`then_0`
                  (`PrimitiveComponent.SetCollisionEnabled` (`self.CapsuleComponent`) "NoCollision")
                  ;[1 1 1] 倒されたら、見えなくして消失エフェクトを表示
                  (`CharacterMovementComponent.DisableMovement` (`self.CharacterMovement`))
                  (`PrimitiveComponent.SetSimulatePhysics` (`self.Mesh`) true)
                  (`PrimitiveComponent.SetSimulatePhysics` (`self.head`) true)
                  (`PrimitiveComponent.SetSimulatePhysics` (`self.wheel`) true)
                  (`KismetSystemLibrary.Delay` 2.0)
                  (`SceneComponent.SetVisibility` (`self.Mesh`) false false)
                  (`SceneComponent.SetVisibility` (`self.head`) false false)
                  (`SceneComponent.SetVisibility` (`self.wheel`) false false)
                  (`NiagaraFunctionLibrary.SpawnSystemAttached` "/Game/bravo/Enemy/VFX/NS_BailOut.NS_BailOut" (`self.Mesh`) "None" (0.0 0.0 0.0) (struct) "SnapToTarget")
                  (`KismetSystemLibrary.Delay` 4.0)
                  (`self.K2_DestroyActor`))
                (:`then_1`
                  ;[1 1 1] 敵を倒したActorに経験値+1
                  (bind _asbp_top_down_character (cast `/Game/TopDown/Blueprints/BP_TopDownCharacter` _returnvalue))
                  (`/Game/TopDown/Blueprints/BP_TopDownCharacter.get_Exp` _asbp_top_down_character)
                  (set `self.isDeath?` true))
                (:`then_2`
                  ;[1 1 1] 敵を倒したら倒した数を更新
                  (bind _asbp_top_down_character_2 (cast `/Game/TopDown/Blueprints/BP_TopDownCharacter` _returnvalue))
                  (`/Game/TopDown/Blueprints/BP_TopDownCharacter.UpdateDefeatsEnemy` _asbp_top_down_character_2)
                  (`KismetSystemLibrary.Delay` 0.5)
                  (goto _label :!via `Reset`)))))
          (:`then_2`
            (bind _returnvalue_2 (`|SpawnActorFromClass` "/Game/bravo/Enemy/BP_DamageText.BP_DamageText_C" (`KismetMathLibrary.Conv_VectorToTransform` (+ (`self.K2_GetActorLocation`) (`KismetMathLibrary.MakeVector` 0.0 0.0 (`KismetMathLibrary.RandomFloatInRange` -20.0 20.0)))) "Undefined" "MultiplyWithRoot" null null))
            (`/Game/bravo/Enemy/BP_DamageText.Ev_BP_DamageText` _returnvalue_2 Damage)))))))

(fn `UserConstructionScript`)