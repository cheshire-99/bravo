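; Game instance Blueprint that handles saving and loading player data through a BPC_GameSave object in a single save slot.
; On Init it creates a new save object only when the slot has no existing save.
; SavePlayerData copies the given data into the cached save reference and writes it to the slot.
; LoadPlayerData reads the slot, caches the cast save object and returns its player data.
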(event `self.ReceiveInit`
  (bind _returnvalue (`GameplayStatics.DoesSaveGameExist` (`self.SaveSlotName`)))
  (if (not _returnvalue)
    (bind _returnvalue_2 (`GameplayStatics.CreateSaveGameObject` "/Game/bravo/Maps/BPC_GameSave.BPC_GameSave_C"))
    (set `self.SaveGameRef` _returnvalue_2)))

(fn `LoadPlayerData`
  (returns (PlayerData :type "/Game/bravo/Maps/PlayerData Structure"))
  (bind _returnvalue (`GameplayStatics.LoadGameFromSlot` (`self.SaveSlotName`)))
  (bind _asbpc_game_save (cast `/Game/bravo/Maps/BPC_GameSave` _returnvalue))
  (bind _output_get (set `self.SaveGameRef` _asbpc_game_save))
  (return (`/Game/bravo/Maps/BPC_GameSave.PlayerData` _output_get)))

(fn `Save Player Data`
  (params (PlayerData :type "/Game/bravo/Maps/PlayerData Structure"))
  (bind _savegameref (`self.SaveGameRef`))
  (set `/Game/bravo/Maps/BPC_GameSave.PlayerData` PlayerData _savegameref)
  (`GameplayStatics.SaveGameToSlot` _savegameref (`self.SaveSlotName`)))